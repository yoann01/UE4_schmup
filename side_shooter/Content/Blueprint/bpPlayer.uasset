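; Player ship for a side-view shooter that flies in the Y/Z plane and fires projectiles.
; A spawn timeline slides and rotates it in, then Tick applies interpolated input movement and pitches the mesh with vertical speed.
; Input gates and cooldowns drive primary, power-up spread and rocket volleys, all spawning Bp_exemple.
; AnyDamage sets Health to clamped Damage minus Health, and at zero flags the game mode and destroys the actor.
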(event Custom|FireRateControl
  (bind _projectilespawn (Variables|Default|GetProjectileSpawn))
  ;[1 1 1] Projectile Control
  (Utilities|FlowControl|Sequence
    (:then_0
      ;;[1 1 1] 0 or less than 0
      (Variables|Float|SetPrimaryFireRate (- (Variables|Float|GetPrimaryFireRate) (Variables|Float|GetDeltaSeconds)))
      (if (<= (Variables|Float|GetPrimaryFireRate) 0.0)
        (Utilities|FlowControl|Gate true
          (:Exit
            (Variables|Float|SetPrimaryFireRate (Variables|Float|GetPrimaryFireRateBase))
            ;;[1 1 1] Checking if P has powerUp
            (if (not (Variables|Default|GetbHasPower))
              (CallFunction|PrimaryFire _projectilespawn)
              (else
                (CallFunction|PowerUpFire (Variables|Default|GetPowerShotCounts) _projectilespawn)))))))
    (:then_1
      (Variables|Float|SetRocketFireRate (- (Variables|Float|GetRocketFireRate) (Variables|Float|GetDeltaSeconds)))
      (if (<= (Variables|Float|GetRocketFireRate) 0.0)
        (Utilities|FlowControl|Gate true
          (:Exit
            (Variables|Float|SetRocketFireRate (Variables|Float|GetRocketFireRateBase))
            (if (Variables|Default|GetbHasRockets)
              (CallFunction|RocketFire (Variables|Default|GetRocketShotCount) _projectilespawn))))))))

(event EventBeginPlay
  ;[1 1 1] SPAWN_ANIMATION
  (Variables|Float|SetHealth (Variables|Float|GetMaxHealth))
  (Variables|Float|SetPitch (.Pitch (Math|Rotator|BreakRotator (Variables|/Script/Engine.SceneComponent|GetRelativeRotation (Variables|Default|GetPlayerMesh)))))
  (Variables|Default|SetSpawnRotation (Transformation|GetWorldRotation (Variables|Default|GetPlayerMesh)))
  (Variables|Default|SetSpawnLocation (Transformation|GetActorLocation))
  (bind _spawn (Timeline|SpawnAnim Play)
    (:Update
      (Transformation|SetActorLocation (Math|Vector|Lerp(Vector) (Variables|Default|GetSpawnLocation) (+ (Variables|Default|GetSpawnLocation) "0,1000.000000, 0") _spawn) false false)
      (Transformation|SetRelativeRotation (Variables|Default|GetPlayerMesh) (Math|Rotator|Lerp(Rotator) (Variables|Default|GetSpawnRotation) (Math|Rotator|MakeRotator 0.0 (+ (Variables|Float|GetAnimationPitch) (Variables|Float|GetPitch)) 0.0) _spawn) false false))
    (:Finished
      (Variables|Default|SetbMovementEnable true))))

(event Collision|EventActorBeginOverlap
  (params (OtherActor :type Actor%20Object%20Reference)))

(event EventTick
  (params (DeltaSeconds :type Float%20%28single-precision%29))
  ;[1 1 1] MOVEMENT
  (Variables|Float|SetDeltaSeconds DeltaSeconds)
  (if (Variables|Default|GetbMovementEnable)
    (CallFunction|FireRateControl)
    (Utilities|FlowControl|Sequence
      (:then_0
        (bind _returndirection (CallFunction|GetDirection (Variables|Float|GetVertSpeed) (Input|AxisValues|GetMoveUp)))
        (Variables|Float|SetVertSpeed _returndirection))
      (:then_1
        (bind _returndirection_2 (CallFunction|GetDirection (Variables|Float|GetHozSpeed) (Input|AxisValues|GetMoveRight)))
        (Variables|Float|SetHozSpeed _returndirection_2))
      (:then_2
        (Transformation|SetActorLocation (+ (Transformation|GetActorLocation) (Math|Vector|MakeVector 0.0 0.0 (stale _output_get))) true false)
        (Transformation|SetActorLocation (+ (Transformation|GetActorLocation) (Math|Vector|MakeVector 0.0 (stale _output_get) 0.0)) true false)
        ;;[0.2338 0.4113 1] Rotation
        (if (> (Variables|Float|GetHealth) 0.0)
          (Transformation|SetRelativeRotation (Variables|Default|GetPlayerMesh) (Math|Interpolation|RInterpTo (Transformation|GetActorRotation) (Math|Rotator|MakeRotator 0.0 (* (Variables|Float|GetVertSpeed) 4.0) 0.0) (Variables|Float|GetDeltaSeconds) 2e+01) false false))))))

(event Game|Damage|EventAnyDamage
  (params (Damage :type Float%20%28single-precision%29) (DamageType :type Damage%20Type%20Object%20Reference) (InstigatedBy :type Controller%20Object%20Reference) (DamageCauser :type Actor%20Object%20Reference))
  (Variables|Float|SetHealth (Math|Float|Clamp(Float) (- Damage (Variables|Float|GetHealth)) 0.0 (Variables|Float|GetMaxHealth)))
  (if (<= (Variables|Float|GetHealth) 0.0)
    (bind _asbp_game_mode (Utilities|Casting|CastTobp_gameMode (Game|GetGameMode)))
    (Variables|/Game/Blueprint/bp_gameMode.bp_gameMode_C|SetpPlayerDead _asbp_game_mode true)
    (Actor|DestroyActor)))

(event Input|ActionEvents|InputActionprimaryFire
  (params (Key :type Key%20Structure :default "AnyKey"))
  (bind _projectilespawn (Variables|Default|GetProjectileSpawn))
  ;[1 1 1] Projectile Control
  (:Pressed
    (Utilities|FlowControl|Gate true) ; enters at Open
  )
  (:Released
    (Utilities|FlowControl|Gate true) ; enters at Close
  ))

(event Input|ActionEvents|InputActionrocketFire
  (params (Key :type Key%20Structure :default "AnyKey"))
  ;[1 1 1] Projectile Control
  (:Pressed
    (Utilities|FlowControl|Gate true) ; enters at Open
  )
  (:Released
    (Utilities|FlowControl|Gate true) ; enters at Close
  ))

(fn ConstructionScript)

(fn GetDirection
  (params (Speed :type Float%20%28single-precision%29) (Direction :type Float%20%28single-precision%29))
  (bind _deltaseconds (Variables|Float|GetDeltaSeconds))
  (bind _output_get (Variables|Float|SetCurrentSpeed (Math|Interpolation|FInterpTo Speed (* (* Direction (Variables|Float|GetMovementSpeed)) _deltaseconds) _deltaseconds 4.0)))
  (return _output_get))

(fn PrimaryFire
  (params (SpawnLocation :type Scene%20Component%20Object%20Reference))
  (bind _returnvalue (Transformation|GetWorldTransform SpawnLocation))
  (bind (_location _rotation) (Math|Transform|BreakTransform _returnvalue))
  (Game|SpawnActorfromClass "/Game/Blueprint/bp_exemple.bp_exemple_C" (Math|Transform|MakeTransform (Math|Vector|MakeVector (.x _location) (.y _location) (+ (.z _location) (Math|Random|RandomFloatinRange -7e+01 7e+01))) _rotation) "AlwaysSpawn" 0 0))

(fn PowerUpFire
  (params (NumberOfShot :type Integer) (SpawnLocation :type Scene%20Component%20Object%20Reference))
  (bind _returnvalue (Transformation|GetWorldTransform SpawnLocation))
  (bind (_location _rotation) (Math|Transform|BreakTransform _returnvalue))
  (LocalVariables|SetOffset (/ NumberOfShot -2))
  (for _index (range 0 NumberOfShot)
    (Game|SpawnActorfromClass "/Game/Blueprint/bp_exemple.bp_exemple_C" (Math|Transform|MakeTransform (Math|Vector|MakeVector (.x _location) (.y _location) (+ (.z _location) (* (Math|Conversions|ToFloat(Integer) (LocalVariables|GetOffset)) 5.0))) (Math|Rotator|MakeRotator (* (Math|Conversions|ToFloat(Integer) (LocalVariables|GetOffset)) 5.0) (.pitch _rotation) (.yaw _rotation))) "AlwaysSpawn" 0 0)
    (LocalVariables|SetOffset (+ (LocalVariables|GetOffset) 1))))

(fn RocketFire
  (params (NumberOfShots :type Integer) (SpawnLocation :type Scene%20Component%20Object%20Reference))
  (bind _returnvalue (Transformation|GetWorldTransform SpawnLocation))
  (bind (_location _rotation) (Math|Transform|BreakTransform _returnvalue))
  (LocalVariables|SetOffset (/ (+ NumberOfShots 1) -1))
  (for _index (range 0 NumberOfShots)
    (Game|SpawnActorfromClass "/Game/Blueprint/bp_exemple.bp_exemple_C" (Math|Transform|MakeTransform (Math|Vector|MakeVector (.x _location) (.y _location) (+ (.z _location) (* (Math|Conversions|ToFloat(Integer) (LocalVariables|GetOffset)) 5.0))) (Math|Rotator|MakeRotator (* (Math|Conversions|ToFloat(Integer) (LocalVariables|GetOffset)) 5.0) (.pitch _rotation) (.yaw _rotation))) "AlwaysSpawn" 0 0)
    (LocalVariables|SetOffset (+ (LocalVariables|GetOffset) 4))))